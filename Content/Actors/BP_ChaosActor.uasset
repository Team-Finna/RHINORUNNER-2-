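; BP_ChaosActor is a breakable cube that rewards the player for running into it.
; On BeginPlay it shifts its Cube by a random X/Y offset.
; When PlayerMain overlaps it, it spawns a BP_FractureCube from the Cube's relative transform, raised slightly, attaches it and wakes its Geometry Collection.
; It then sends score and boredom ("Bordem") amounts to the player and hides itself without being destroyed.
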(event `self.ReceiveBeginPlay`
  (bind _returnvalue (`KismetMathLibrary.RandomFloatInRange` -200.0 200.0))
  (bind _cube (`self.Cube`))
  (bind (_relativelocation_x _relativelocation_y _relativelocation_z) (`KismetMathLibrary.BreakVector` (`SceneComponent.RelativeLocation` _cube)))
  (`SceneComponent.K2_SetRelativeLocation` _cube (`KismetMathLibrary.MakeVector` (+ _relativelocation_x _returnvalue) (+ _returnvalue _relativelocation_y) _relativelocation_z) false false))

(event `self.ReceiveActorBeginOverlap`
  (params (OtherActor :type "Actor Object Reference"))
  (bind (_returnvalue_location _returnvalue_rotation _returnvalue_scale) (`KismetMathLibrary.BreakTransform` (`SceneComponent.GetRelativeTransform` (`self.Cube`))))
  (bind _asplayer_main (cast `/Game/Rhino/PlayerFolder/PlayerMain` OtherActor))
  (bind _returnvalue (`|SpawnActorFromClass` "/Game/Actors/BP_FractureCube.BP_FractureCube_C" (`KismetMathLibrary.MakeTransform` (+ _returnvalue_location (0.0 0.0 60.0)) _returnvalue_rotation _returnvalue_scale) "Undefined" "MultiplyWithRoot" null null))
  (`self.K2_AttachToComponent` _returnvalue (`self.Cube`) "None" "KeepWorld" "KeepRelative" "KeepRelative" true)
  (`PrimitiveComponent.WakeRigidBody` (`GeometryCollectionActor.GeometryCollectionComponent` _returnvalue) "None")
  (message `/Game/UISystems/PlayerToUI.AddScore` _asplayer_main 200.0)
  (message `/Game/UISystems/PlayerToUI.AddBordem` _asplayer_main 2000.0)
  (`self.SetActorHiddenInGame` true))

(fn `UserConstructionScript`)