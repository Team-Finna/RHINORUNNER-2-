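; BP_Falling is an actor that stays hidden in game until the player character comes within range.
; BeginPlay hides it, then Tick measures the distance from the player's mesh world location to the StaticMesh's relative location, not its world location.
; Below a fixed threshold it unhides the actor and never hides it again.
; The graph contains no falling logic.
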(event `self.ReceiveBeginPlay`
  (`self.SetActorHiddenInGame` true))

(event `self.ReceiveTick`
  (params (DeltaSeconds :type "Float (single-precision)"))
  (bind _returnvalue_location (`KismetMathLibrary.BreakTransform` (`SceneComponent.GetRelativeTransform` (`self.StaticMesh`))))
  (if (< (`KismetMathLibrary.Vector_Distance` (`SceneComponent.K2_GetComponentLocation` (`Character.Mesh` (`GameplayStatics.GetPlayerCharacter` 0))) _returnvalue_location) 2000.0)
    (`self.SetActorHiddenInGame` false)))

(fn `UserConstructionScript`)